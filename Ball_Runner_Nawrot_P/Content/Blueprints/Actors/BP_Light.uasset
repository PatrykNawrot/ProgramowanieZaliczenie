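; BP_Light is a light actor with two spotlights that switch on temporarily when the player overlaps it.
; Both spotlights start at zero intensity on BeginPlay, and a player overlap raises them to a fixed high intensity.
; A Delay then turns both off after 22 seconds; re-entering during that time does not extend the countdown.
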(event EventBeginPlay
  (Rendering|Components|Light|SetIntensity (Variables|Default|GetSpotLight) 0.0)
  (Rendering|Components|Light|SetIntensity (Variables|Default|GetSpotLight1) 0.0))

(event Collision|EventActorBeginOverlap
  (params (OtherActor :type Actor%20Object%20Reference))
  (Utilities|IsPlayer OtherActor
    (:IsPlayer
      (Rendering|Components|Light|SetIntensity (Variables|Default|GetSpotLight) 66193.828125)
      (Rendering|Components|Light|SetIntensity (Variables|Default|GetSpotLight1) 66193.828125)
      (Utilities|FlowControl|Delay 22.0)
      (Rendering|Components|Light|SetIntensity (Variables|Default|GetSpotLight) 0.0)
      (Rendering|Components|Light|SetIntensity (Variables|Default|GetSpotLight1) 0.0))))

(event EventTick
  (params (DeltaSeconds :type Float%20%28single-precision%29)))

(fn ConstructionScript)