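; BP_BackToStart is an actor that sends the player back to a start location when they overlap it while crystals remain in the level.
; On overlap, an IsPlayer check filters the other actor, then CheckAnyCrystals counts all BP_Crystal actors and returns true only when none are left.
; If any remain, it sets the player pawn's relative location to StartLocation without sweep or teleport.
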(event EventBeginPlay)

(event Collision|EventActorBeginOverlap
  (params (OtherActor :type Actor%20Object%20Reference))
  (Utilities|IsPlayer OtherActor
    (:IsPlayer
      (if (not (Pure|CheckAnyCrystals))
        (Transformation|SetActorRelativeLocation (Game|Player|GetPlayerPawn 0) (Variables|Default|GetStartLocation))))))

(event EventTick
  (params (DeltaSeconds :type Float%20%28single-precision%29)))

(fn ConstructionScript)

(fn CheckAnyCrystals
  (bind _outactors (Actor|GetAllActorsOfClass "/Game/Blueprints/Actors/Collectables/BP_Crystal.BP_Crystal_C"))
  (return (== (Utilities|Array|Length _outactors) 0)))