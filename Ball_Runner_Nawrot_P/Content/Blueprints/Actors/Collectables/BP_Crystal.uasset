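; Collectable crystal that spins in place and gets drawn into the player on overlap, then disappears.
; A player-only overlap caches its location, scale and light intensity, then plays the TL_BlendAlpha timeline.
; The timeline lerps it toward the player's live position while shrinking it and fading its point light, then destroys it.
; Tick adds a fixed yaw step each frame, so spin speed depends on frame rate.
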(event EventTick
  (params (DeltaSeconds :type Float%20%28single-precision%29))
  (Transformation|SetActorRotation (Math|Rotator|MakeRotator 0.0 0.0 (+ (.yaw (Transformation|GetActorRotation)) 1.0))))

(event Collision|EventActorBeginOverlap
  (params (OtherActor :type Actor%20Object%20Reference))
  (Utilities|IsPlayer OtherActor
    (:IsPlayer
      (CallFunction|StartLocation)
      (CallFunction|StartScale)
      (CallFunction|StartIntensity)
      (bind (_direction _smoothlerpalpha _scale _lightintensity) (Timeline|TL_BlendAlpha Play)
        (:Update
          (CallFunction|GetCrystaltoPlayer _smoothlerpalpha)
          (CallFunction|GetCrystalSmall _scale)
          (CallFunction|ChangeIntensity _lightintensity))
        (:Finished
          (Actor|DestroyActor))))))

(fn ConstructionScript)

(fn GetCrystaltoPlayer
  (params (Alpha :type Float%20%28single-precision%29))
  (Transformation|SetActorLocation (Math|Vector|Lerp(Vector) (Variables|Default|GetLerpStartLocation) (Transformation|GetActorLocation (Game|Player|GetPlayerPawn 0)) Alpha) false false))

(fn StartLocation
  (Variables|Default|SetLerpStartLocation (Transformation|GetActorLocation)))

(fn StartScale
  (Variables|Default|SetLerpStartScale (Transformation|GetActorScale3D)))

(fn GetCrystalSmall
  (params (Alpha :type Float%20%28single-precision%29))
  (Transformation|SetActorScale3D (Math|Vector|Lerp(Vector) (Variables|Default|GetLerpStartScale) "0, 0, 0" Alpha)))

(fn StartIntensity
  (Variables|Default|SetLerpStartIntensity (Variables|/Script/Engine.LightComponentBase|GetIntensity (Variables|Default|GetPointLight))))

(fn ChangeIntensity
  (params (Alpha :type Float%20%28single-precision%29))
  (Rendering|Components|Light|SetIntensity (Variables|Default|GetPointLight) (Math|Float|Lerp (Variables|Default|GetLerpStartIntensity) 0.0 Alpha)))