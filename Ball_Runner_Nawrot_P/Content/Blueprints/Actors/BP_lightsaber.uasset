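; BP_lightsaber is a laser hazard actor that damages the player on overlap.
; When IsMovable is set, BeginPlay stores its location and a timeline lerps its Z from that height toward a fixed world height.
; A delay chained to the timeline's update replays it from the start, looping the motion.
; Overlap with the player applies a small fixed damage to player pawn 0, whether the hazard moves or not.
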(event EventBeginPlay
  (if (Variables|Default|GetIsMovable)
    (Variables|Default|SetLerpStartLocationLaser (Transformation|GetActorLocation))
    (bind _z_location (Timeline|MoveLightsaber Play)
      (:Update
        (Transformation|SetActorLocation (Math|Vector|MakeVector (.x (Variables|Default|GetLerpStartLocationLaser)) (.y (Variables|Default|GetLerpStartLocationLaser)) (Math|Float|Lerp (.z (Variables|Default|GetLerpStartLocationLaser)) 1e+02 _z_location)) false false)
        (Utilities|FlowControl|Delay 3.2)
        (Timeline|MoveLightsaber PlayFromStart)))))

(event Collision|EventActorBeginOverlap
  (params (OtherActor :type Actor%20Object%20Reference))
  (Utilities|IsPlayer OtherActor
    (:IsPlayer
      (Game|Damage|ApplyDamage (Game|Player|GetPlayerPawn 0) 2.0 0 0))))

(event EventTick
  (params (DeltaSeconds :type Float%20%28single-precision%29)))

(fn ConstructionScript)