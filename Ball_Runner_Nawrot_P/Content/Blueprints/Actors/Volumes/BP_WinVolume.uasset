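; BP_WinVolume is a level-exit volume that completes the level when the player overlaps it and no BP_Crystal actors remain in the world.
; The crystal check runs only at overlap time, by counting all actors of that class.
; Completion looks up the current level name in the LevelNames array, then opens the following entry or quits the game if it is the last.
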(event EventBeginPlay)

(event Collision|EventActorBeginOverlap
  (params (OtherActor :type Actor%20Object%20Reference))
  (Utilities|IsPlayer OtherActor
    (:IsPlayer
      (if (Pure|CheckAnyCrystals)
        (Impure|CompleteLevel)))))

(event EventTick
  (params (DeltaSeconds :type Float%20%28single-precision%29)))

(fn ConstructionScript)

(fn CheckAnyCrystals
  (bind _outactors (Actor|GetAllActorsOfClass "/Game/Blueprints/Actors/Collectables/BP_Crystal.BP_Crystal_C"))
  (return (== (Utilities|Array|Length _outactors) 0)))

(fn CompleteLevel
  (if (Pure|IsFinalLvl)
    (Game|QuitGame 0 "Quit")
    (else
      (Game|OpenLevel(byName) (Pure|GetNextLevelName)))))

(fn GetCurrentLevelIndex
  (bind _returnvalue (Game|GetCurrentLevelName true))
  (return (Utilities|Array|FindItem (Variables|Default|GetLevelNames) (Utilities|String|StringToName _returnvalue))))

(fn GetLastLevelIndex
  (return (Utilities|Array|LastIndex (Variables|Default|GetLevelNames))))

(fn IsFinalLvl
  (return (== (Pure|GetLastLevelIndex) (Pure|GetCurrentLevelIndex))))

(fn GetNextLevelName
  (bind _returnvalue (Game|GetCurrentLevelName true))
  (return (Utilities|Array|Get(acopy) (Variables|Default|GetLevelNames) (+ (Utilities|Array|FindItem (Variables|Default|GetLevelNames) (Utilities|String|StringToName _returnvalue)) 1))))