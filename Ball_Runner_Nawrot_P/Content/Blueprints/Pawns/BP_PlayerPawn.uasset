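; Player pawn that moves its static mesh with physics torque and restarts the level when damaged.
; Both movement axes feed one AddTorqueInRadians node, applying input scaled by TorqueStrenght on X and Y as an acceleration change.
; Any damage calls the ResetLevel macro, which fades the camera out, waits, then reopens the current level by name.
; Escape quits the game.
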(event EventBeginPlay)

(event Collision|EventActorBeginOverlap
  (params (OtherActor :type Actor%20Object%20Reference)))

(event EventTick
  (params (DeltaSeconds :type Float%20%28single-precision%29)))

(event Game|Damage|EventAnyDamage
  (params (Damage :type Float%20%28single-precision%29) (DamageType :type Damage%20Type%20Object%20Reference) (InstigatedBy :type Controller%20Object%20Reference) (DamageCauser :type Actor%20Object%20Reference))
  (Utilities|ResetLevel))

(event Input|AxisEvents|InputAxisMoveForward/Backwards
  (params (AxisValue :type Float%20%28single-precision%29))
  (bind _torquestrenght (Variables|Default|GetTorqueStrenght))
  (Class|PrimitiveComponent|AddTorqueinRadians (Variables|Default|GetStaticMesh) (Math|Vector|MakeVector (* (stale Input|AxisEvents|InputAxisMoveLeft/Righ AxisValue) _torquestrenght) (* AxisValue _torquestrenght) 0.0) "None" true))

(event Input|AxisEvents|InputAxisMoveLeft/Righ
  (params (AxisValue :type Float%20%28single-precision%29))
  (bind _torquestrenght (Variables|Default|GetTorqueStrenght))
  (Class|PrimitiveComponent|AddTorqueinRadians (Variables|Default|GetStaticMesh) (Math|Vector|MakeVector (* AxisValue _torquestrenght) (* (stale Input|AxisEvents|InputAxisMoveForward/Backwards AxisValue) _torquestrenght) 0.0) "None" true))

(event Input|KeyboardEvents|Escape
  (params (Key :type Key%20Structure))
  (:Pressed
    (Game|QuitGame 0 "Quit")))

(fn ConstructionScript)